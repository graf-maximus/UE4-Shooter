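; Weapon pickup spawner that gives its displayed weapon to an overlapping player character and respawns a replacement after a delay.
; The Construction Script creates the initial weapon as a collision-disabled child actor of the configured class.
; On sphere overlap, the server passes that actor to the player's weapon manager if they lack that weapon type.
; A timer then spawns a new weapon actor above the spawner.
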(event OnComponentBeginOverlap(Sphere)
  (params (OverlappedComponent :type Primitive%20Component%20Object%20Reference) (OtherActor :type Actor%20Object%20Reference) (OtherComp :type Primitive%20Component%20Object%20Reference) (OtherBodyIndex :type Integer) (bFromSweep :type Boolean) (SweepResult :type Hit%20Result%20Structure%20%28by%20ref%29))
  (Networking|SwitchHasAuthority
    (:Authority
      (bind _asbp_player_character (Utilities|Casting|CastToBP_PlayerCharacter OtherActor))
      (bind _currentweapon (Variables|Default|GetCurrentWeapon)
        (:then
          (if (not (Default|HasWeaponbyType (Variables|/Game/Blueprints/Players/BP_PlayerCharacter.BP_PlayerCharacter_C|GetBP_WeaponManager _asbp_player_character) (Variables|/Game/Blueprints/Weapon/BP_Weapon.BP_Weapon_C|GetWeaponType (Variables|Default|GetCurrentWeapon))))
            (Default|AddWeapon (Variables|/Game/Blueprints/Players/BP_PlayerCharacter.BP_PlayerCharacter_C|GetBP_WeaponManager _asbp_player_character) _currentweapon)
            (Variables|Default|SetCurrentWeapon 0)
            (Utilities|Time|SetTimerbyFunctionName 0 "RespawnWeapon" (Variables|Default|GetRespawnTime))))
        (:else)))))

(fn ConstructionScript
  (bind _returnvalue (AddComponent|AddChildActorComponent false))
  (ChildActorComponent|SetChildActorClass _returnvalue (Variables|Default|GetWeaponClass))
  (bind _output_get (Variables|Default|SetCurrentWeapon (.AsBP%20Weapon (Utilities|Casting|CastToBP_Weapon (Variables|/Script/Engine.ChildActorComponent|GetChildActor _returnvalue)))))
  (Collision|SetActorEnableCollision _output_get false))

(fn RespawnWeapon
  (bind _returnvalue (Game|SpawnActorfromClass (Variables|Default|GetWeaponClass) (Math|Transform|MakeTransform (+ (Transformation|GetActorLocation) "0, 0,100.000000") "0, 0, 0" "1,1,1") "Undefined" 0 0 0))
  (Variables|Default|SetCurrentWeapon _returnvalue))