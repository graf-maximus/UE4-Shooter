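; Team variant of the game mode, adding two-team assignment, team scoring and team rules on top of its parent.
; Join-in-progress players go to the smaller team, and random players switch sides to even out teams before match start.
; Spawns use free player starts matching the player's team, and damage respects the friendly-fire setting.
; Kills award points to the instigator's team in BP_TeamGameState, optionally stopping the match at a limit.
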(event EventOnPlayerConnected
  (params (PlayerState :type BP%20Player%20State%20Object%20Reference))
  (if (Variables|Default|GetAllowJoinInProgress)
    (|SendPlayerInTeam PlayerState)
    (|CallParentFunction PlayerState)))

(fn ConstructionScript
  (|CallParentFunction))

(fn GetFreeSpawnPoints
  (params (Player :type BP%20Player%20Controller%20Object%20Reference))
  (bind _outactors (Actor|GetAllActorsOfClass "/Game/Blueprints/Game/BP_PlayerStart.BP_PlayerStart_C"))
  (for _array_element _outactors
    (if (and (Default|IsFree _array_element) (== (Variables|/Game/Blueprints/Game/BP_PlayerStart.BP_PlayerStart_C|GetTeam _array_element) (Variables|/Game/Blueprints/Game/BP_TeamPlayerState.BP_TeamPlayerState_C|GetTeam (.AsBP%20Team%20Player%20State (Utilities|Casting|CastToBP_TeamPlayerState (Variables|/Script/Engine.Controller|GetPlayerState Player))))))
      (Utilities|Array|Add (LocalVariables|GetL_Starts) _array_element)))
  (return (LocalVariables|GetL_Starts)))

(fn UpdateDeathPoints
  (params (Player :type BP%20Player%20Controller%20Object%20Reference) (Instigator :type BP%20Player%20Controller%20Object%20Reference))
  (|CallParentFunction Player Instigator)
  (Default|AddTeamPoints (.AsBP%20Team%20Game%20State (Utilities|Casting|CastToBP_TeamGameState (Game|GetGameState))) (Variables|/Game/Blueprints/Game/BP_TeamPlayerState.BP_TeamPlayerState_C|GetTeam (.AsBP%20Team%20Player%20State (Utilities|Casting|CastToBP_TeamPlayerState (Variables|/Script/Engine.Controller|GetPlayerState Instigator)))) 1))

(fn ShouldDamagePlayer?
  (params (DamagedPlayer :type BP%20Player%20Controller%20Object%20Reference) (Instigator :type BP%20Player%20Controller%20Object%20Reference))
  (Utilities|IsValid Instigator
    (:Is%20Valid
      (if (Variables|Default|GetAllowFriendlyFire)
        (return true)
        (else
          (return (!= (Variables|/Game/Blueprints/Game/BP_TeamPlayerState.BP_TeamPlayerState_C|GetTeam (.AsBP%20Team%20Player%20State (Utilities|Casting|CastToBP_TeamPlayerState (Variables|/Script/Engine.Controller|GetPlayerState DamagedPlayer)))) (Variables|/Game/Blueprints/Game/BP_TeamPlayerState.BP_TeamPlayerState_C|GetTeam (.AsBP%20Team%20Player%20State (Utilities|Casting|CastToBP_TeamPlayerState (Variables|/Script/Engine.Controller|GetPlayerState Instigator)))))))))
    (:Is%20Not%20Valid
      (return true))))

(fn CharacterDead
  (params (KilledCharacter :type BP%20Player%20Character%20Object%20Reference) (DeathInstigator :type BP%20Player%20Controller%20Object%20Reference) (DeathCausedBy :type Actor%20Object%20Reference))
  (|CallParentFunction KilledCharacter DeathInstigator DeathCausedBy)
  (if (Variables|Default|GetLimitByTeamPoints)
    (if (>= (Default|GetTeamPoints (.AsBP%20Team%20Game%20State (Utilities|Casting|CastToBP_TeamGameState (Game|GetGameState))) (Variables|/Game/Blueprints/Game/BP_TeamPlayerState.BP_TeamPlayerState_C|GetTeam (.AsBP%20Team%20Player%20State (Utilities|Casting|CastToBP_TeamPlayerState (Variables|/Script/Engine.Controller|GetPlayerState DeathInstigator))))) (Variables|Default|GetTeamPointsLimit))
      (CallFunction|StopMatch "Limit by team points"))))

(fn BalanceTeams
  (bind _returnvalue (Game|GetGameState))
  (bind _l_teamaplayers (LocalVariables|GetL_TeamAPlayers))
  (bind _l_teambplayers (LocalVariables|GetL_TeamBPlayers))
  (bind _returnvalue_2 (> _l_teamaplayers _l_teambplayers))
  (bind _asbp_team_game_state (Utilities|Casting|CastToBP_TeamGameState _returnvalue))
  (bind _returnvalue_3 (select _returnvalue_2 "NewEnumerator0" "NewEnumerator1"))
  (bind _players (Default|GetTeamPlayers _asbp_team_game_state _returnvalue_3))
  (|GetTeamsPlayersNumber)
  (bind _playersnum (|NeedsToBalance)
    (:true
      (for _index (range 1 (/ _playersnum 2))
        (Variables|/Game/Blueprints/Game/BP_TeamPlayerState.BP_TeamPlayerState_C|SetTeam (Utilities|Array|Get(acopy) _players (Math|Random|RandomInteger (Utilities|Array|Length _players))) (select (> (LocalVariables|GetL_TeamAPlayers) (LocalVariables|GetL_TeamBPlayers)) "NewEnumerator1" "NewEnumerator0"))))))

(fn StartMatch
  (CallFunction|BalanceTeams)
  (|CallParentFunction))