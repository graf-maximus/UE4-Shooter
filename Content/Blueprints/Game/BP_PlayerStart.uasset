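; BP_PlayerStart is a spawn point that creates player characters and tracks whether its spot is occupied.
; SpawnCharacter spawns a BP_PlayerCharacter at its transform, has the given player possess it, and fires CharacterSpawned.
; The spawned or most recently overlapping character is stored as CharacterInside and cleared when that character leaves the capsule.
; IsFree reports the spot as available only when no valid character is stored.
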(event OnComponentBeginOverlap(CapsuleComponent)
  (params (OverlappedComponent :type Primitive%20Component%20Object%20Reference) (OtherActor :type Actor%20Object%20Reference) (OtherComp :type Primitive%20Component%20Object%20Reference) (OtherBodyIndex :type Integer) (bFromSweep :type Boolean) (SweepResult :type Hit%20Result%20Structure%20%28by%20ref%29))
  (bind _asbp_player_character (Utilities|Casting|CastToBP_PlayerCharacter OtherActor))
  (Variables|Default|SetCharacterInside _asbp_player_character))

(event OnComponentEndOverlap(CapsuleComponent)
  (params (OverlappedComponent :type Primitive%20Component%20Object%20Reference) (OtherActor :type Actor%20Object%20Reference) (OtherComp :type Primitive%20Component%20Object%20Reference) (OtherBodyIndex :type Integer))
  (if (== OtherActor (Variables|Default|GetCharacterInside))
    (Variables|Default|SetCharacterInside 0)))

(fn ConstructionScript)

(fn SpawnCharacter
  (params (Player :type BP%20Player%20Controller%20Object%20Reference))
  (bind _returnvalue (Game|SpawnActorfromClass "/Game/Blueprints/Players/BP_PlayerCharacter.BP_PlayerCharacter_C" (Transformation|GetActorTransform) "Undefined" Player 0))
  (bind _output_get (Variables|Default|SetCharacterInside _returnvalue))
  (Pawn|Possess Player _output_get)
  (Default|CallCharacterSpawned Player)
  (return _returnvalue))

(fn IsFree
  (Variables|Default|GetCharacterInside
    (:then
      (return false))
    (:else
      (return true))))