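; Game mode that runs a match: spawning players, handling deaths and ending play, with optional time limit and join-in-progress.
; Players spawn at random free BP_PlayerStart points on match start or when joining mid-game.
; Deaths update kills and deaths, optionally start a respawn timer, and possess a spectator pawn following the killer, or free-flying without one.
; Dispatchers announce deaths and match start/end; ShouldDamagePlayer always allows damage.
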(event EventBeginPlay
  (EventDispatchers|AssignPlayerConnected (.AsBP%20Game%20State%20Base (Utilities|Casting|CastToBP_GameStateBase (Game|GetGameState))) (EventDispatchers|CreateEvent :!event OnPlayerConnected)))

(fn ConstructionScript)

(fn CharacterDead
  (params (KilledCharacter :type BP%20Player%20Character%20Object%20Reference) (DeathInstigator :type BP%20Player%20Controller%20Object%20Reference) (DeathCausedBy :type Actor%20Object%20Reference))
  (LocalVariables|SetL_KilledChar KilledCharacter)
  (LocalVariables|SetL_DeathCausedBy DeathCausedBy)
  (LocalVariables|SetL_DeathInstigator DeathInstigator)
  (Default|CallCharDead (LocalVariables|GetL_KilledChar) (LocalVariables|GetL_DeathInstigator) (LocalVariables|GetL_DeathCausedBy))
  (Utilities|FlowControl|Sequence
    (:then_0
      (CallFunction|UpdateDeathPoints (.AsBP%20Player%20Controller (Utilities|Casting|CastToBP_PlayerController (Pawn|GetController (LocalVariables|GetL_KilledChar)))) (LocalVariables|GetL_DeathInstigator)))
    (:then_1
      (Default|OwnerCharDead (.AsBP%20Player%20State (Utilities|Casting|CastToBP_PlayerState (Variables|/Script/Engine.Pawn|GetPlayerState (LocalVariables|GetL_KilledChar)))) (.AsBP%20Player%20Character (Utilities|Casting|CastToBP_PlayerCharacter (Pawn|GetControlledPawn (LocalVariables|GetL_DeathInstigator)))) (LocalVariables|GetL_DeathCausedBy)))
    (:then_2
      (Utilities|FlowControl|Sequence
        (:then_0
          (if (Variables|Default|GetAutoRespawn)
            (Default|LaunchRespawnTimer (.AsBP%20Player%20Controller (Utilities|Casting|CastToBP_PlayerController (Pawn|GetController (LocalVariables|GetL_KilledChar)))) (Variables|Default|GetRespawnTime))))
        (:then_1
          (CallFunction|SpawnSpectator (.AsBP%20Player%20Controller (Utilities|Casting|CastToBP_PlayerController (Pawn|GetController (LocalVariables|GetL_KilledChar)))) (LocalVariables|GetL_DeathInstigator)))))))

(fn SpawnPlayer
  (params (Player :type BP%20Player%20Controller%20Object%20Reference))
  (bind _returnvalue (Pawn|GetControlledPawn Player))
  (Utilities|IsValid _returnvalue
    (:Is%20Valid
      (Actor|DestroyActor _returnvalue))
    (:Is%20Not%20Valid
      _))
  (bind _spawns (CallFunction|GetFreeSpawnPoints Player))
  (bind _output_get (LocalVariables|SetL_PlayerStart (Utilities|Array|Get(acopy) _spawns (Math|Random|RandomInteger (Utilities|Array|LastIndex _spawns)))))
  (Default|SpawnCharacter _output_get Player)
  (Variables|/Game/Blueprints/Game/BP_PlayerState.BP_PlayerState_C|SetIs%20alive? (.AsBP%20Player%20State (Utilities|Casting|CastToBP_PlayerState (Variables|/Script/Engine.Controller|GetPlayerState Player))) true))

(fn GetFreeSpawnPoints
  (params (Player :type BP%20Player%20Controller%20Object%20Reference))
  (bind _outactors (Actor|GetAllActorsOfClass "/Game/Blueprints/Game/BP_PlayerStart.BP_PlayerStart_C"))
  (for _array_element _outactors
    (if (Default|IsFree _array_element)
      (Utilities|Array|Add (LocalVariables|GetL_Starts) _array_element)))
  (return (LocalVariables|GetL_Starts)))

(fn SpawnSpectator
  (params (Player :type BP%20Player%20Controller%20Object%20Reference) (DeathInstigator :type BP%20Player%20Controller%20Object%20Reference))
  (LocalVariables|SetL_Player Player)
  (bind _output_get (LocalVariables|SetL_Instigator DeathInstigator))
  (Utilities|IsValid _output_get
    (:Is%20Valid
      (bind _returnvalue (Game|SpawnActorfromClass "/Game/Blueprints/Game/Spectator/BP_SpectatorPawn_ForCharacter.BP_SpectatorPawn_ForCharacter_C" (Transformation|GetActorTransform (Pawn|GetControlledPawn (LocalVariables|GetL_Player))) "Undefined" 0 (LocalVariables|GetL_Player) 0))
      (LocalVariables|SetL_Spectator _returnvalue)
      (Variables|/Game/Blueprints/Game/Spectator/BP_SpectatorPawn_ForCharacter.BP_SpectatorPawn_ForCharacter_C|SetFollowCharacter _returnvalue (.AsBP%20Player%20Character (Utilities|Casting|CastToBP_PlayerCharacter (Pawn|GetControlledPawn (LocalVariables|GetL_Instigator))))))
    (:Is%20Not%20Valid
      (bind _returnvalue_2 (Game|SpawnActorfromClass "/Game/Blueprints/Game/Spectator/BP_SpectatorPawn_Free.BP_SpectatorPawn_Free_C" (Transformation|GetActorTransform (Pawn|GetControlledPawn (LocalVariables|GetL_Player))) "Undefined" 0 (LocalVariables|GetL_Player) 0))
      (bind _output_get_2 (LocalVariables|SetL_Spectator _returnvalue_2))))
  (Pawn|Possess (LocalVariables|GetL_Player) (LocalVariables|GetL_Spectator))
  (return _output_get_2))

(fn StartMatch
  (for _array_element (Variables|/Script/Engine.GameStateBase|GetPlayerArray (Game|GetGameState))
    (bind _asbp_player_controller (Utilities|Casting|CastToBP_PlayerController (Components|GetOwner _array_element)))
    (CallFunction|SpawnPlayer _asbp_player_controller))
  (Default|CallMatchStarted))

(fn UpdateDeathPoints
  (params (Player :type BP%20Player%20Controller%20Object%20Reference) (Instigator :type BP%20Player%20Controller%20Object%20Reference))
  (Default|AddDeaths (.AsBP%20Player%20State (Utilities|Casting|CastToBP_PlayerState (Variables|/Script/Engine.Controller|GetPlayerState Player))))
  (Default|AddKills (.AsBP%20Player%20State (Utilities|Casting|CastToBP_PlayerState (Variables|/Script/Engine.Controller|GetPlayerState Instigator)))))

(fn StopMatch
  (params (StopReason :type String))
  (for _array_element (Variables|/Script/Engine.GameStateBase|GetPlayerArray (Game|GetGameState))
    (bind _asbp_player_controller (Utilities|Casting|CastToBP_PlayerController (Components|GetOwner _array_element)))
    (CallFunction|SpawnSpectator _asbp_player_controller))
  (bind _outactors (Actor|GetAllActorsOfClass "/Game/Blueprints/Players/BP_PlayerCharacter.BP_PlayerCharacter_C"))
  (Actor|DestroyActor _outactors)
  (Default|CallMatchEnded StopReason))

(fn TimeLimitReached
  (if (Variables|Default|GetLimitByTime)
    (CallFunction|StopMatch "TimeLimit")))

(fn ShouldDamagePlayer?
  (params (DamagedPlayer :type BP%20Player%20Controller%20Object%20Reference) (Instigator :type BP%20Player%20Controller%20Object%20Reference))
  (return true))

(fn OnPlayerConnected
  (params (PlayerState :type BP%20Player%20State%20Object%20Reference))
  (switch Utilities|FlowControl|Switch|SwitchonE_MatchState (Variables|/Game/Blueprints/Game/BP_GameStateBase.BP_GameStateBase_C|GetRoundInProgress (.AsBP%20Game%20State%20Base (Utilities|Casting|CastToBP_GameStateBase (Game|GetGameState))))
    (:NewEnumerator1
      (if (Variables|Default|GetAllowJoinInProgress)
        (bind _asbp_player_controller (Utilities|Casting|CastToBP_PlayerController (Components|GetOwner PlayerState)))
        (CallFunction|SpawnPlayer _asbp_player_controller)))))