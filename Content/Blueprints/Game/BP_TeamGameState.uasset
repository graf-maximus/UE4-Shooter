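; Game state for a two-team mode that tracks each team's score and looks up its players.
; BeginPlay sizes a points array from the TeamPoints map, and AddTeamPoints updates both in parallel.
; GetTeamPoints reads only the array, mapping TeamA and TeamB to indices.
; GetTeamPlayers filters PlayerArray by the Team stored on each BP_TeamPlayerState.
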(event EventBeginPlay
  (|CallParentFunction)
  (Utilities|Array|Resize (Variables|Default|GetTeamPointsArray) (Utilities|Map|Length (Variables|Default|GetTeamPoints))))

(fn ConstructionScript
  (|CallParentFunction))

(fn AddTeamPoints
  (params (Team :type E_Teams%20Enum :default "NewEnumerator0") (Points :type Integer))
  (bind _returnvalue (Utilities|Select :Index Team :NewEnumerator0 0 :NewEnumerator1 1))
  (bind _teampoints (Variables|Default|GetTeamPoints))
  (Utilities|Map|Add _teampoints Team (+ (.Value (Utilities|Map|Find _teampoints Team)) Points))
  (Utilities|Array|SetArrayElem (Variables|Default|GetTeamPointsArray) _returnvalue (+ (Utilities|Array|Get(acopy) (Variables|Default|GetTeamPointsArray) _returnvalue) Points)))

(fn GetTeamPoints
  (params (Team :type E_Teams%20Enum :default "NewEnumerator0"))
  (return (Utilities|Array|Get(acopy) (Variables|Default|GetTeamPointsArray) (Utilities|Select :Index Team :NewEnumerator0 0 :NewEnumerator1 1))))

(fn GetTeamPlayers
  (params (Team :type E_Teams%20Enum :default "NewEnumerator0"))
  (for _array_element (Variables|Default|GetPlayerArray)
    (bind _asbp_team_player_state (Utilities|Casting|CastToBP_TeamPlayerState _array_element))
    (if (Utilities|Enum|Equal(Enum) (Variables|/Game/Blueprints/Game/BP_TeamPlayerState.BP_TeamPlayerState_C|GetTeam _asbp_team_player_state) Team)
      (Utilities|Array|Add (LocalVariables|GetL_Players) _asbp_team_player_state)))
  (return (LocalVariables|GetL_Players)))