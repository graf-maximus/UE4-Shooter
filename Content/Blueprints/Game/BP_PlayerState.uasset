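; Player state Blueprint that tracks a player's kills, deaths and alive status.
; Two seconds after BeginPlay it registers itself with BP_GameStateBase as a newly connected player.
; Owner character death clears IsAlive and fires the PlayerDead dispatcher with instigator, death causer and itself.
; IsAlive uses a RepNotify that fires PlayerAlive when it turns true, while simple functions increment the kill and death counters.
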(event Custom|OwnerCharDead
  (params (Instigator :type BP%20Player%20Character%20Object%20Reference) (Death%20Causer :type Actor%20Object%20Reference))
  (Variables|Default|SetIs%20alive? false)
  (Default|CallPlayerDead Instigator Death%20Causer self))

(event EventBeginPlay
  (Utilities|FlowControl|Delay 2.0)
  (Default|NewPlayerConnected (.AsBP%20Game%20State%20Base (Utilities|Casting|CastToBP_GameStateBase (Game|GetGameState))) self))

(fn ConstructionScript)

(fn AddKills
  (Math|Integer|IncrementInt (Variables|Default|GetKills)))

(fn AddDeaths
  (Math|Integer|IncrementInt (Variables|Default|GetDeaths)))

(fn OnRepIsAlive?
  (if (Variables|Default|GetIs%20alive?)
    (Default|CallPlayerAlive)))