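; Main HUD that switches the player's screens across pre-start, live play, spectating and post-match stats, alongside a persistent chat widget.
; GameState match events and PlayerState alive/dead events drive Toggle functions, which lazily create and reuse each widget.
; Tab menu and spectator toggles are gated on the round state, and spectating receives killer and weapon info.
; Showing a screen also switches input between game-only and UI-only with cursor.
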(event Custom|OnMatchStarted
  (bind _returnvalue (Game|Player|GetOwningPlayerController))
  (bind _playerstate (Variables|/Script/Engine.Controller|GetPlayerState _returnvalue))
  (bind _asbp_player_state (Utilities|Casting|CastToBP_PlayerState _playerstate))
  (CallFunction|TogglePreStart false)
  (CallFunction|ToggleMainHUD true)
  (EventDispatchers|AssignPlayerAlive _asbp_player_state (delegate Custom|OnPlayerAlive))
  (EventDispatchers|AssignPlayerDead _asbp_player_state (delegate Custom|OnPlayerDead)))

(event Custom|OnPlayerAlive
  (CallFunction|ToggleMainHUD true)
  (CallFunction|ToggleSpectatorHUD false))

(event Custom|OnMatchEnded
  (CallFunction|ToggleMainHUD false)
  (CallFunction|ToggleTabMenu false)
  (CallFunction|ToggleSpectatorHUD false)
  (CallFunction|TogglePostStatsMenu true))

(event Custom|OnPlayerDead
  (params (Instigator :type BP%20Player%20Character%20Object%20Reference) (DeathCauser :type Actor%20Object%20Reference) (PlayerState :type BP%20Player%20State%20Object%20Reference))
  (CallFunction|ToggleMainHUD false)
  (CallFunction|ToggleSpectatorHUD true)
  (if (Utilities|Enum|Equal(Enum) (Variables|/Game/Blueprints/Game/BP_GameStateBase.BP_GameStateBase_C|GetRoundInProgress (.AsBP%20Game%20State%20Base (Utilities|Casting|CastToBP_GameStateBase (Game|GetGameState)))) "NewEnumerator1")
    (Default|SetInfo (Variables|Default|GetSpectatorHUD) Instigator DeathCauser)))

(event EventBeginPlay
  (bind _returnvalue (Game|GetGameState))
  (bind _asbp_game_state_base (Utilities|Casting|CastToBP_GameStateBase _returnvalue))
  (CallFunction|CreateChat)
  (CallFunction|TogglePreStart true)
  (EventDispatchers|AssignMatchStarted _asbp_game_state_base (delegate Custom|OnMatchStarted))
  (EventDispatchers|AssignMatchEnded _asbp_game_state_base (delegate Custom|OnMatchEnded)))

(fn ConstructionScript)

(fn ToggleMainHUD
  (params (Show :type Boolean))
  (if Show
    (if (Variables|/Game/Blueprints/Game/BP_PlayerState.BP_PlayerState_C|GetIs%20alive? (.AsBP%20Player%20State (Utilities|Casting|CastToBP_PlayerState (Variables|/Script/Engine.Controller|GetPlayerState (Game|Player|GetOwningPlayerController)))))
      (bind _mainhud (Variables|Default|GetMainHUD)
        (:then
          (UserInterface|Viewport|AddtoViewport _mainhud 0))
        (:else
          (bind _returnvalue (UserInterface|CreateWidget (Variables|Default|GetMainHUDClass) (Game|Player|GetOwningPlayerController)))
          (bind _output_get (Variables|Default|SetMainHUD _returnvalue))
          (UserInterface|Viewport|AddtoViewport _output_get 0)))
      (CallFunction|SetInputUIMode false))
    (else
      (bind _mainhud_2 (Variables|Default|GetMainHUD)
        (:then
          (Widget|RemovefromParent _mainhud_2))
        (:else)))))

(fn ToggleTabMenu
  (params (Show :type Boolean))
  (if (Utilities|Enum|Equal(Enum) (Variables|/Game/Blueprints/Game/BP_GameStateBase.BP_GameStateBase_C|GetRoundInProgress (.AsBP%20Game%20State%20Base (Utilities|Casting|CastToBP_GameStateBase (Game|GetGameState)))) "NewEnumerator1")
    (if Show
      (bind _tabmenu (Variables|Default|GetTabMenu)
        (:then
          (UserInterface|Viewport|AddtoViewport _tabmenu 0))
        (:else
          (bind _returnvalue (UserInterface|CreateWidget (Variables|Default|GetTabMenuClass) (Game|Player|GetOwningPlayerController)))
          (bind _output_get (Variables|Default|SetTabMenu _returnvalue))
          (UserInterface|Viewport|AddtoViewport _output_get 0)))
      (CallFunction|SetInputUIMode false)
      (else
        (bind _tabmenu_2 (Variables|Default|GetTabMenu)
          (:then
            (Widget|RemovefromParent _tabmenu_2))
          (:else))))))

(fn ToggleSpectatorHUD
  (params (Show :type Boolean))
  (if (Utilities|Enum|Equal(Enum) (Variables|/Game/Blueprints/Game/BP_GameStateBase.BP_GameStateBase_C|GetRoundInProgress (.AsBP%20Game%20State%20Base (Utilities|Casting|CastToBP_GameStateBase (Game|GetGameState)))) "NewEnumerator1")
    (if Show
      (bind _spectatorhud (Variables|Default|GetSpectatorHUD)
        (:then
          (UserInterface|Viewport|AddtoViewport _spectatorhud 0))
        (:else
          (bind _returnvalue (UserInterface|CreateWidget (Variables|Default|GetSpectatorHUDClass) (Game|Player|GetOwningPlayerController)))
          (bind _output_get (Variables|Default|SetSpectatorHUD _returnvalue))
          (UserInterface|Viewport|AddtoViewport _output_get 0)))
      (CallFunction|SetInputUIMode false)
      (else
        (bind _spectatorhud_2 (Variables|Default|GetSpectatorHUD)
          (:then
            (Widget|RemovefromParent _spectatorhud_2))
          (:else))))))

(fn TogglePreStart
  (params (Show :type Boolean))
  (if Show
    (bind _prestarthud (Variables|Default|GetPreStartHUD)
      (:then
        (UserInterface|Viewport|AddtoViewport _prestarthud 0))
      (:else
        (bind _returnvalue (UserInterface|CreateWidget (Variables|Default|GetPreStartHUDClass) (Game|Player|GetOwningPlayerController)))
        (bind _output_get (Variables|Default|SetPreStartHUD _returnvalue))
        (UserInterface|Viewport|AddtoViewport _output_get 0)))
    (CallFunction|SetInputUIMode true (Variables|Default|GetPreStartHUD))
    (else
      (bind _prestarthud_2 (Variables|Default|GetPreStartHUD)
        (:then
          (Widget|RemovefromParent _prestarthud_2))
        (:else)))))

(fn TogglePostStatsMenu
  (params (Show :type Boolean))
  (if Show
    (bind _poststatshud (Variables|Default|GetPostStatsHUD)
      (:then
        (UserInterface|Viewport|AddtoViewport _poststatshud 0))
      (:else
        (bind _returnvalue (UserInterface|CreateWidget (Variables|Default|GetPostStatsHUDClass) (Game|Player|GetOwningPlayerController)))
        (bind _output_get (Variables|Default|SetPostStatsHUD _returnvalue))
        (UserInterface|Viewport|AddtoViewport _output_get 0)))
    (CallFunction|SetInputUIMode true (Variables|Default|GetPostStatsHUD))
    (else
      (bind _poststatshud_2 (Variables|Default|GetPostStatsHUD)
        (:then
          (Widget|RemovefromParent _poststatshud_2))
        (:else)))))

(fn CreateChat
  (bind _returnvalue (UserInterface|CreateWidget (Variables|Default|GetChatMenuClass) (Game|Player|GetOwningPlayerController)))
  (bind _output_get (Variables|Default|SetChatMenu _returnvalue))
  (UserInterface|Viewport|AddtoViewport _output_get 0))

(fn ToggleSpeakChat
  (params (Activate :type Boolean))
  (bind _chatmenu (Variables|Default|GetChatMenu))
  (if Activate
    (Default|ActivateChat _chatmenu)
    (else
      (Default|DeactivateChat _chatmenu))))

(fn SetInputUIMode
  (params (UI :type Boolean) (WidgetToFocus :type User%20Widget%20Object%20Reference))
  (bind _returnvalue (Game|Player|GetOwningPlayerController))
  (if UI
    (Variables|/Script/Engine.PlayerController|SetbShowMouseCursor _returnvalue true)
    (Input|SetInputModeUIOnly _returnvalue WidgetToFocus "DoNotLock")
    (else
      (Variables|/Script/Engine.PlayerController|SetbShowMouseCursor _returnvalue false)
      (Input|SetInputModeGameOnly _returnvalue))))