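; BP_PlayerGameMode_Deathmatch is a deathmatch game mode that ends the match once a player reaches the kill limit.
; It extends the inherited CharacterDead handler, calling the parent first, then reading the instigator's kill count from BP_PlayerState.
; When that count meets or exceeds KillsLimit, it calls StopMatch with "KillLimit" as the reason.
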(event EventBeginPlay
  (|CallParentFunction) ; This node is disabled and will not be called.\nDrag off pins to build functionality.
)

(event EventTick
  (params (DeltaSeconds :type Float%20%28single-precision%29))
  (|CallParentFunction DeltaSeconds) ; This node is disabled and will not be called.\nDrag off pins to build functionality.
)

(event EventCharacterDead
  (params (KilledCharacter :type BP%20Player%20Character%20Object%20Reference) (DeathInstigator :type BP%20Player%20Controller%20Object%20Reference) (DeathCausedBy :type Actor%20Object%20Reference))
  (|CallParentFunction KilledCharacter DeathInstigator DeathCausedBy)
  (if (>= (Variables|/Game/Blueprints/Game/BP_PlayerState.BP_PlayerState_C|GetKills (.AsBP%20Player%20State (Utilities|Casting|CastToBP_PlayerState (Variables|/Script/Engine.Controller|GetPlayerState DeathInstigator)))) (Variables|Default|GetKillsLimit))
    (CallFunction|StopMatch "KillLimit")))

(fn ConstructionScript
  (|CallParentFunction))