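; BP_TeamPlayerState is a player state that randomly assigns each player to one of two teams.
; On BeginPlay, only the authority picks the Team value and copies it to the owning BP_TeamPlayerController.
; The parent BeginPlay runs only on that authority path, after the controller cast succeeds.
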(event EventBeginPlay
  (Networking|SwitchHasAuthority
    (:Authority
      (Variables|Default|SetTeam (Utilities|Select :Index (Math|Random|RandomInteger 2) :Option%200 "NewEnumerator0" :Option%201 "NewEnumerator1"))
      (bind _asbp_team_player_controller (Utilities|Casting|CastToBP_TeamPlayerController (Components|GetOwner)))
      (Variables|/Game/Blueprints/Players/BP_TeamPlayerController.BP_TeamPlayerController_C|SetTeam _asbp_team_player_controller (Variables|Default|GetTeam))
      (|CallParentFunction))))

(fn ConstructionScript
  (|CallParentFunction))