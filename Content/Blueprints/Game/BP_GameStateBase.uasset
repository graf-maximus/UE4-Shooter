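; Game state that runs the match round lifecycle: pre-start countdown, timed play, end of match and map vote.
; A one-second server tick counts down once enough players join, starts the match through BP_PlayerGameMode, then tracks play time against its time limit.
; Match end is multicast and opens a BPMapVoteComponent vote, whose DT_VoteMaps result triggers ServerTravel.
; RoundInProgress's RepNotify fires match start and end dispatchers.
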(event Custom|OnMatchEnded
  (params (StopReason :type String))
  (CallFunction|MulticastonMatchEnded StopReason)
  (Variables|Default|SetRoundInProgress "NewEnumerator2")
  (Default|StartVote (Variables|Default|GetBP_MapVoteComponent))
  (EventDispatchers|AssignVoteEnded (Variables|Default|GetBP_MapVoteComponent) (delegate Custom|OnVoteEnded)))

(event Custom|Multicast_OnMatchEnded
  (params (StopReason :type String))
  (Default|CallTimeEnded StopReason))

(event Custom|OnVoteEnded
  (params (NewMap :type Name))
  (bind _returnvalue (Utilities|GetDataTableRow "/Game/Data/DataTable/DT_VoteMaps.DT_VoteMaps" NewMap)
    (:then
      (CallFunction|StartServerNewMap (.MapName (Utilities|Struct|BreakS_MapInfo _returnvalue))))))

(event EventBeginPlay
  (Networking|SwitchHasAuthority
    (:Authority
      (bind _asbp_player_game_mode (Utilities|Casting|CastToBP_PlayerGameMode (Game|GetGameMode)))
      (EventDispatchers|AssignMatchEnded _asbp_player_game_mode (delegate Custom|OnMatchEnded)))))

(event EventTick
  (params (DeltaSeconds :type Float%20%28single-precision%29))
  (Networking|SwitchHasAuthority
    (:Authority
      (switch Utilities|FlowControl|Switch|SwitchonE_MatchState (Variables|Default|GetRoundInProgress)
        (:NewEnumerator0
          (if (>= (Utilities|Array|Length (Variables|Default|GetPlayerArray)) (Variables|Default|GetPlayersAmountForStart))
            (bind _result (Math|Integer|DecrementInt (Variables|Default|GetPreStartTime))
              (:%20%20
                (if (<= _result 0)
                  (Default|StartMatch (.AsBP%20Player%20Game%20Mode (Utilities|Casting|CastToBP_PlayerGameMode (Game|GetGameMode))))
                  (Variables|Default|SetRoundInProgress "NewEnumerator1"))))
            (else
              (Variables|Default|SetPreStartTime (.PreStartTime (Utilities|GetClassDefaults (Utilities|GetClass self)))))))
        (:NewEnumerator1
          (CallFunction|PlayTimeTick))))))

(fn ConstructionScript)

(fn PlayTimeTick
  (bind _output_get (Variables|Default|SetPlayTime (+ (Math|Timespan|MakeTimespan 0 0 0 1) (Variables|Default|GetPlayTime))))
  (Variables|Default|SetMinutes (.Minutes (Math|Timespan|BreakTimespan _output_get)))
  (Variables|Default|SetSeconds (.Seconds (Math|Timespan|BreakTimespan _output_get)))
  (bind _asbp_player_game_mode (Utilities|Casting|CastToBP_PlayerGameMode (Game|GetGameMode)))
  (if (and (>= (Variables|Default|GetPlayTime) (Variables|/Game/Blueprints/Game/BP_PlayerGameMode.BP_PlayerGameMode_C|GetTimeLimit _asbp_player_game_mode)) (Utilities|Enum|Equal(Enum) (Variables|Default|GetRoundInProgress) "NewEnumerator1"))
    (Default|TimeLimitReached (.AsBP%20Player%20Game%20Mode (Utilities|Casting|CastToBP_PlayerGameMode (Game|GetGameMode))))))

(fn GetRoundTime
  (return (Variables|Default|GetMinutes) (Variables|Default|GetSeconds)))

(fn OnRepRoundinProgress
  (switch Utilities|FlowControl|Switch|SwitchonE_MatchState (Variables|Default|GetRoundInProgress)
    (:NewEnumerator1
      (Default|CallMatchStarted))
    (:NewEnumerator2
      (Default|CallMatchEnded))))

(fn GetPreRoundTime
  (return (Variables|Default|GetPreStartTime)))

(fn StartServerNewMap
  (params (Map :type Name))
  (Development|ExecuteConsoleCommand (Utilities|String|Append "ServerTravel " (Utilities|String|ToString(Name) Map)) 0))

(fn NewPlayerConnected
  (params (PlayerState :type BP%20Player%20State%20Object%20Reference))
  (Default|CallPlayerConnected PlayerState))