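; Spectator pawn that follows a character's position while letting the player rotate the view through Turn and LookUp axis input.
; On non-authority instances only, Tick interpolates the pawn's location toward FollowCharacter with VInterpTo whenever that reference is valid.
; BeginPlay on those instances waits a second before setting the interpolation speed used for the follow.
; FollowCharacter is not assigned within this Blueprint's graphs.
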(event EventBeginPlay
  (Networking|SwitchHasAuthority
    (:Remote
      (Utilities|FlowControl|Delay 1.0)
      (Variables|Default|SetInterpSpeed 2e+01))))

(event EventTick
  (params (DeltaSeconds :type Float%20%28single-precision%29))
  (Networking|SwitchHasAuthority
    (:Remote
      (bind _followcharacter (Variables|Default|GetFollowCharacter)
        (:then
          (Transformation|SetActorLocation (Math|Interpolation|VInterpTo (Transformation|GetActorLocation) (Transformation|GetActorLocation _followcharacter) (Utilities|Time|GetWorldDeltaSeconds) (Variables|Default|GetInterpSpeed)) false false))
        (:else)))))

(event Input|AxisEvents|InputAxisLookUp
  (params (AxisValue :type Float%20%28single-precision%29))
  (Pawn|Input|AddControllerPitchInput AxisValue))

(event Input|AxisEvents|InputAxisTurn
  (params (AxisValue :type Float%20%28single-precision%29))
  (Pawn|Input|AddControllerYawInput AxisValue))

(fn ConstructionScript
  (|CallParentFunction))