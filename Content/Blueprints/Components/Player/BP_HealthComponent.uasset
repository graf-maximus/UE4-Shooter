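; Player character component that tracks health and armour and handles death from incoming damage.
; On the server it binds to the owner's damage event and asks the game mode whether the instigator may hurt a living player.
; Math expressions scale damage by armour and update both values.
; At zero health it marks the character dead and reports the victim, instigating controller and damage causer to the game mode.
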(event Custom|OnPlayerTakeAnyDamage
  (params (DamagedActor :type Actor%20Object%20Reference) (Damage :type Float%20%28single-precision%29) (DamageType :type Damage%20Type%20Object%20Reference) (InstigatedBy :type Controller%20Object%20Reference) (DamageCauser :type Actor%20Object%20Reference))
  (|ShouldDamagePlayer InstigatedBy)
  (CallFunction|ApplyDamage Damage)
  (if (and (<= (Variables|Default|GetHealth) 0.0) (not (Variables|/Game/Blueprints/Players/BP_PlayerCharacter.BP_PlayerCharacter_C|GetDead (Variables|Default|GetCharacter))))
    (Variables|/Game/Blueprints/Players/BP_PlayerCharacter.BP_PlayerCharacter_C|SetDead (Variables|Default|GetCharacter) true)
    (bind _asbp_player_game_mode (Utilities|Casting|CastToBP_PlayerGameMode (Game|GetGameMode)))
    (Default|CharacterDead _asbp_player_game_mode (Variables|Default|GetCharacter) (.AsBP%20Player%20Controller (Utilities|Casting|CastToBP_PlayerController InstigatedBy)) DamageCauser)))

(event EventBeginPlay
  (Variables|Default|SetHealth (Variables|Default|GetMaxHealth))
  (Variables|Default|SetArmour (Variables|Default|GetMaxArmour))
  (bind _asbp_player_character (Utilities|Casting|CastToBP_PlayerCharacter (Components|GetOwner)))
  (bind _output_get (Variables|Default|SetCharacter _asbp_player_character))
  (if (Networking|IsServer)
    (EventDispatchers|AssignOnTakeAnyDamage _output_get (EventDispatchers|CreateEvent :!event Custom|OnPlayerTakeAnyDamage))))

(fn ApplyDamage
  (params (Damage :type Float%20%28single-precision%29))
  (LocalVariables|SetL_Damage (|(Damage*(1-({701CD6BD-4D65-0DCC-2AB3-0DA272365483}/200))) Damage))
  (Variables|Default|SetHealth (- (Variables|Default|GetHealth) (LocalVariables|GetL_Damage)))
  (Variables|Default|SetArmour (|(max(({701CD6BD-4D65-0DCC-2AB3-0DA272365483}-({259D3548-4629-5288-F232-04883B1DD64A}*2.000000)),0)))))

(fn GetHealth
  (return (Variables|Default|GetHealth) (Variables|Default|GetMaxHealth)))

(fn GetArmour
  (return (Variables|Default|GetArmour) (Variables|Default|GetMaxArmour)))