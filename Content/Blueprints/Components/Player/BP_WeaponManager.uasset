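; Player weapon manager component that holds main, secondary and melee slots plus specials and grenade arrays.
; Creates, adds, selects and drops weapons by type; dropping destroys the actor and switches to another weapon.
; Scrolling flattens all slots into one list and steps through it with wrap-around.
; CurrentWeapon's OnRep attaches the weapon to the visible mesh socket on clients, hides the previous one and signals the selection.
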(event Custom|SelectWeaponFromClient
  (params (Type :type E_WeaponType%20Enum :default "NewEnumerator0") (Index :type Integer) (Weapon :type BP%20Weapon%20Object%20Reference))
  ;[1 1 1] Switch weapon
  (CallFunction|SelectWeapon Type Index Weapon))

(event Custom|DropWeaponFromClient
  (Variables|Default|GetCurrentWeapon
    (:then
      (CallFunction|ServerDropWeapon))
    (:else)))

(event Custom|ServerDropWeapon
  (bind _currentweapon (Variables|Default|GetCurrentWeapon)
    (:then
      (CallFunction|DropWeapon _currentweapon))
    (:else)))

(event Custom|ScrollWeaponOnClient
  (params (Next :type Boolean))
  ;[1 1 1] Switch weapon
  (bind (_success _weapon) (CallFunction|ScrollWeapon Next))
  (if _success
    (CallFunction|SelectWeaponfromClient "NewEnumerator0" 0 _weapon)))

(event EventBeginPlay
  (bind _asbp_player_character (Utilities|Casting|CastToBP_PlayerCharacter (Components|GetOwner)))
  (Variables|Default|SetCharacter _asbp_player_character))

(fn CreateWeapon
  (params (Actor%20Class :type BP%20Weapon%20Class%20Reference))
  (bind _character (Variables|Default|GetCharacter))
  (bind _returnvalue (Game|SpawnActorfromClass Actor%20Class (Math|Transform|MakeTransform "0, 0, 0" "0, 0, 0" "1,1,1") "AlwaysSpawn" (Pawn|GetController _character) _character _character))
  (bind _output_get (LocalVariables|SetL_Weapon _returnvalue))
  (switch Utilities|FlowControl|Switch|SwitchonE_WeaponType (Variables|/Game/Blueprints/Weapon/BP_Weapon.BP_Weapon_C|GetWeaponType _output_get)
    (:NewEnumerator0
      (Variables|Default|SetMainWeapon (LocalVariables|GetL_Weapon)))
    (:NewEnumerator1
      (Variables|Default|SetSecondaryWeapon (LocalVariables|GetL_Weapon)))
    (:NewEnumerator2
      (Variables|Default|SetMeleeWeapon (.AsBP%20Melee%20Weapons (Utilities|Casting|CastToBP_MeleeWeapons (LocalVariables|GetL_Weapon)))))
    (:NewEnumerator3
      (Utilities|Array|Add (Variables|Default|GetSpecials) (LocalVariables|GetL_Weapon)))
    (:NewEnumerator4
      (Utilities|Array|Add (Variables|Default|GetGrenades) (LocalVariables|GetL_Weapon))))
  (Transformation|AttachActorToActor (LocalVariables|GetL_Weapon) (Variables|Default|GetCharacter) "None" "SnapToTarget" "SnapToTarget" "KeepRelative" true)
  (return (LocalVariables|GetL_Weapon)))

(fn OnRepCurrentWeapon
  (Utilities|FlowControl|Sequence
    (:then_0
      (if (not (Networking|IsServer))
        (bind _currentweapon (Variables|Default|GetCurrentWeapon)
          (:then
            (Rendering|SetActorHiddenInGame _currentweapon false)
            (bind _clientweaponattached (Variables|Default|GetClientWeaponAttached)
              (:then
                (Transformation|AttachActorToActor _clientweaponattached (Variables|Default|GetCharacter) "None" "SnapToTarget" "SnapToTarget" "KeepRelative" true)
                (Rendering|SetActorHiddenInGame (Variables|Default|GetClientWeaponAttached) true))
              (:else
                _))
            (bind _currentweapon_2 (Variables|Default|GetCurrentWeapon)
              (:then
                (Transformation|AttachComponentToComponent _currentweapon_2 (Default|GetVisibleMesh (Variables|Default|GetCharacter)) "Skt_Weapon" "SnapToTarget" "SnapToTarget" "KeepRelative" true)
                (Variables|Default|SetClientWeaponAttached (Variables|Default|GetCurrentWeapon)))
              (:else)))
          (:else
            (Variables|Default|SetClientWeaponAttached 0)))))
    (:then_1
      (Default|CallWeaponSelected (Variables|Default|GetCurrentWeapon)))))

(fn SelectWeapon
  (params (WeaponType :type E_WeaponType%20Enum :default "NewEnumerator0") (Index :type Integer) (Weapon :type BP%20Weapon%20Object%20Reference))
  (bind _specials (Variables|Default|GetSpecials))
  (bind _grenades (Variables|Default|GetGrenades))
  (bind _mainweapon (Variables|Default|GetMainWeapon))
  (bind _secondaryweapon (Variables|Default|GetSecondaryWeapon))
  (bind _meleeweapon (Variables|Default|GetMeleeWeapon))
  (bind _output (Utilities|Array|Get(acopy) _grenades Index))
  (bind _output_2 (Utilities|Array|Get(acopy) _specials Index))
  (bind _returnvalue (Utilities|Select :Index WeaponType :NewEnumerator0 _mainweapon :NewEnumerator1 _secondaryweapon :NewEnumerator2 _meleeweapon :NewEnumerator3 _output_2 :NewEnumerator4 _output))
  (Utilities|IsValid Weapon
    (:Is%20Valid
      (bind _output_get (Variables|Default|SetCurrentWeapon Weapon))
      (return _output_get))
    (:Is%20Not%20Valid
      (Utilities|IsValid _returnvalue
        (:Is%20Valid
          (bind _output_get_2 (Variables|Default|SetCurrentWeapon _returnvalue))
          (return _output_get_2))
        (:Is%20Not%20Valid
          (return 0))))))

(fn AddWeapon
  (params (Weapon :type BP%20Weapon%20Object%20Reference))
  (bind _output_get (LocalVariables|SetL_Weapon Weapon))
  (CallFunction|DropWeapon (Utilities|Select :Index (Variables|/Game/Blueprints/Weapon/BP_Weapon.BP_Weapon_C|GetWeaponType _output_get) :NewEnumerator0 (Variables|Default|GetMainWeapon) :NewEnumerator1 (Variables|Default|GetSecondaryWeapon) :NewEnumerator2 (Variables|Default|GetMeleeWeapon) :NewEnumerator3 (Utilities|Array|Get(acopy) (Variables|Default|GetSpecials)) :NewEnumerator4 (Utilities|Array|Get(acopy) (Variables|Default|GetGrenades))))
  (switch Utilities|FlowControl|Switch|SwitchonE_WeaponType (Variables|/Game/Blueprints/Weapon/BP_Weapon.BP_Weapon_C|GetWeaponType _output_get)
    (:NewEnumerator0
      (Variables|Default|SetMainWeapon (LocalVariables|GetL_Weapon)))
    (:NewEnumerator1
      (Variables|Default|SetSecondaryWeapon (LocalVariables|GetL_Weapon)))
    (:NewEnumerator2
      (Variables|Default|SetMeleeWeapon (.AsBP%20Melee%20Weapons (Utilities|Casting|CastToBP_MeleeWeapons (LocalVariables|GetL_Weapon)))))
    (:NewEnumerator3
      (Utilities|Array|Add (Variables|Default|GetSpecials) (LocalVariables|GetL_Weapon)))
    (:NewEnumerator4
      (Utilities|Array|Add (Variables|Default|GetGrenades) (LocalVariables|GetL_Weapon))))
  (Variables|/Game/Blueprints/Weapon/BP_Weapon.BP_Weapon_C|SetWeaponOwner (LocalVariables|GetL_Weapon) (Variables|Default|GetCharacter))
  (bind _currentweapon (Variables|Default|GetCurrentWeapon)
    (:then)
    (:else
      (Variables|Default|SetCurrentWeapon _currentweapon))))

(fn DropWeapon
  (params (Weapon :type BP%20Weapon%20Object%20Reference))
  (Utilities|IsValid Weapon
    (:Is%20Valid
      (bind _output_get (LocalVariables|SetL_Weapon Weapon))
      (if (== (Variables|/Game/Blueprints/Weapon/BP_Weapon.BP_Weapon_C|GetWeaponOwner _output_get) (Variables|Default|GetCharacter))
        (bind _weapon (CallFunction|ScrollWeapon true))
        (Variables|Default|SetCurrentWeapon _weapon)
        (switch Utilities|FlowControl|Switch|SwitchonE_WeaponType (Variables|/Game/Blueprints/Weapon/BP_Weapon.BP_Weapon_C|GetWeaponType (LocalVariables|GetL_Weapon))
          (:NewEnumerator0
            (Variables|Default|SetMainWeapon 0))
          (:NewEnumerator1
            (Variables|Default|SetSecondaryWeapon 0))
          (:NewEnumerator2
            (Variables|Default|SetMeleeWeapon 0))
          (:NewEnumerator3
            (Utilities|Array|RemoveItem (Variables|Default|GetSpecials) (LocalVariables|GetL_Weapon)))
          (:NewEnumerator4
            (Utilities|Array|RemoveItem (Variables|Default|GetGrenades) (LocalVariables|GetL_Weapon))))
        (Variables|/Game/Blueprints/Weapon/BP_Weapon.BP_Weapon_C|SetWeaponOwner (LocalVariables|GetL_Weapon) 0)
        (Actor|DestroyActor (LocalVariables|GetL_Weapon))
        (bind _weapon_2 (CallFunction|ScrollWeapon true))
        (Variables|Default|SetCurrentWeapon _weapon_2)))))

(fn ScrollWeapon
  (params (Next :type Boolean))
  (bind _weapon (|SetWeaponFromArray))
  (bind _l_weapons (LocalVariables|GetL_Weapons))
  (bind _currentweapon (Variables|Default|GetCurrentWeapon))
  (bind _returnvalue (Utilities|Array|FindItem _l_weapons _currentweapon))
  (LocalVariables|SetL_Next Next)
  (|MakeWeaponsArray)
  (if (> (Utilities|Array|Length (LocalVariables|GetL_Weapons)) 1)
    (if (>= _returnvalue 0)
      (LocalVariables|SetL_Index _returnvalue)
      (Utilities|IsValid _weapon
        (:Is%20Valid
          (return true _weapon))))
    (else
      (return false 0))))

(fn HasWeaponbyType
  (params (Index :type E_WeaponType%20Enum :default "NewEnumerator0"))
  (Utilities|IsValid (Utilities|Select :Index Index :NewEnumerator0 (Variables|Default|GetMainWeapon) :NewEnumerator1 (Variables|Default|GetSecondaryWeapon) :NewEnumerator2 (Variables|Default|GetMeleeWeapon) :NewEnumerator3 (Utilities|Array|Get(acopy) (Variables|Default|GetSpecials)) :NewEnumerator4 (Utilities|Array|Get(acopy) (Variables|Default|GetGrenades)))
    (:Is%20Valid
      (return true))
    (:Is%20Not%20Valid
      (return false))))