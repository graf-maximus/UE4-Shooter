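; Map vote component that runs a timed vote among randomly picked maps from a data table.
; StartVote draws maps without repeats from DT_VoteMaps and enables tick, which decrements VoteTime until StopVote.
; SetVote stores each player's choice by GameState PlayerArray index and updates the leading map.
; RepNotifies on the map list and in-progress flag broadcast list changes, vote start, and the winning map at end.
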(event EventTick
  (params (DeltaSeconds :type Float%20%28single-precision%29))
  (bind _result (Math|Float|DecrementFloat (Variables|Default|GetVoteTime))
    (:%20%20
      (if (<= _result 0.0)
        (CallFunction|StopVote)))))

(fn OnRepVoteinProgress
  (if (Variables|Default|GetVoteInProgress)
    (Default|CallVoteStarted)
    (else
      (Default|CallVoteEnded (Utilities|Array|Get(acopy) (Variables|Default|GetMaps) (CallFunction|GetVotedMap))))))

(fn StartVote
  (Components|Tick|SetComponentTickEnabled true)
  (CallFunction|ChooseMapstoVote)
  (Variables|Default|SetVoteInProgress true))

(fn StopVote
  (Variables|Default|SetVoteInProgress false)
  (Components|Tick|SetComponentTickEnabled false))

(fn ChooseMapstoVote
  (Utilities|Array|Clear (Variables|Default|GetMaps))
  (bind _outrownames (DataTable|GetDataTableRowNames "/Game/Data/DataTable/DT_VoteMaps.DT_VoteMaps"))
  (LocalVariables|SetL_Maps _outrownames)
  (for _index (range 1 (Variables|Default|GetNumberOfMaps))
    (if (> (Utilities|Array|Length (LocalVariables|GetL_Maps)) 0)
      (LocalVariables|SetL_RandomMapIndex (Math|Random|RandomInteger (Utilities|Array|Length (LocalVariables|GetL_Maps))))
      (Utilities|Array|Add (Variables|Default|GetMaps) (Utilities|Array|Get(acopy) (LocalVariables|GetL_Maps) (LocalVariables|GetL_RandomMapIndex)))
      (Utilities|Array|RemoveIndex (LocalVariables|GetL_Maps) (LocalVariables|GetL_RandomMapIndex))
      (else
        (return))))
  (return))

(fn GetVotedMap
  (for (_ _array_index) (Variables|Default|GetMaps)
    (Utilities|Array|Add (LocalVariables|GetL_Votes) (CallFunction|GetMapVotes _array_index)))
  (return (.IndexOfMaxValue (Math|Integer|MaxOfIntArray (LocalVariables|GetL_Votes)))))

(fn SetVote
  (params (MapIndex :type Integer) (Player :type BP%20Player%20State%20Object%20Reference))
  (Utilities|Array|SetArrayElem (Variables|Default|GetPlayersVotes) (Utilities|Array|FindItem (Variables|/Script/Engine.GameStateBase|GetPlayerArray (Game|GetGameState)) Player) MapIndex true)
  (Variables|Default|SetMaxVotesMap (CallFunction|GetVotedMap)))

(fn GetMapVotes
  (params (MapIndex :type Integer))
  (for _array_element (Variables|Default|GetPlayersVotes)
    (if (== _array_element MapIndex)
      (Math|Integer|IncrementInt (LocalVariables|GetL_Votes))))
  (return (LocalVariables|GetL_Votes)))

(fn GetMaps
  (return (Variables|Default|GetMaps)))

(fn OnRepMaps
  (Default|CallMapVoteChanged (Variables|Default|GetMaps)))