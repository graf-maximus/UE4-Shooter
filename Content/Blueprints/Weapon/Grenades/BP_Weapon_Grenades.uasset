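; Grenade weapon Blueprint that throws a projectile when used.
; UseWeapon runs the parent's check, then calls ThrowProjectile only on the authority, so spawning is server-side.
; ThrowProjectile spawns the FireProjectile class just ahead of the instigating player character's camera, aimed along the owner's forward vector with a fixed rotation offset, and passes it Damage and the instigator.
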(event EventBeginPlay
  (|CallParentFunction) ; This node is disabled and will not be called.\nDrag off pins to build functionality.
)

(event Collision|EventActorBeginOverlap
  (params (OtherActor :type Actor%20Object%20Reference))
  (|CallParentFunction OtherActor) ; This node is disabled and will not be called.\nDrag off pins to build functionality.
)

(event EventTick
  (params (DeltaSeconds :type Float%20%28single-precision%29))
  (|CallParentFunction DeltaSeconds) ; This node is disabled and will not be called.\nDrag off pins to build functionality.
)

(fn ConstructionScript
  (|CallParentFunction))

(fn UseWeapon
  (bind _used (|CallParentFunction))
  (if _used
    (Networking|SwitchHasAuthority
      (:Authority
        (CallFunction|ThrowProjectile)
        (return true)))
    (else
      (return false))))

(fn ThrowProjectile
  (bind _asbp_player_character (Utilities|Casting|CastToBP_PlayerCharacter (Game|GetInstigator)))
  (Game|SpawnActorfromClass (Variables|Default|GetFireProjectile) (Math|Transform|MakeTransform (+ (Transformation|GetWorldLocation (Variables|/Game/Blueprints/Players/BP_PlayerCharacter.BP_PlayerCharacter_C|GetCamera _asbp_player_character)) (* (Transformation|GetActorForwardVector (Components|GetOwner)) 50)) (Math|Rotator|CombineRotators (Math|Conversions|RotationFromXVector (Transformation|GetActorForwardVector (Components|GetOwner))) "10.000000, 0, 0") "1,1,1") "AlwaysSpawn" self (Variables|Default|GetDamage) (Game|GetInstigator)))