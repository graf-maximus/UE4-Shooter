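; Grenade projectile for the weapon system that bounces as a physics body and explodes after a timed fuse.
; On BeginPlay the authority launches the capsule forward with a random spin and starts the Explosion timer.
; Explosion deals full radial damage, blockable by WorldStatic geometry, then destroys the actor.
; The destruction itself triggers the explosion particle effect, spawned only on remote instances without an RPC.
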(event EventBeginPlay
  (Networking|SwitchHasAuthority
    (:Authority
      (Physics|AddImpulse (Variables|Default|GetCapsule) (* (Transformation|GetActorForwardVector) 3e+03) "None" false)
      (Class|PrimitiveComponent|AddAngularImpulseinDegrees (Variables|Default|GetCapsule) (Math|Vector|MakeVector (Math|Random|RandomFloatinRange -5e+02 5e+02) (Math|Random|RandomFloatinRange -5e+02 5e+02) (Math|Random|RandomFloatinRange -5e+02 5e+02)) "None" false)
      (Utilities|Time|SetTimerbyFunctionName 0 "Explosion" (Variables|Default|GetExplosionTime)))))

(event EventDestroyed
  (|CallParentFunction)
  (Networking|SwitchHasAuthority
    (:Remote
      (Effects|SpawnEmitteratLocation "/Game/StarterContent/Particles/P_Explosion.P_Explosion" (Transformation|GetActorLocation)))))

(fn ConstructionScript
  (|CallParentFunction))

(fn Explosion
  (Game|Damage|ApplyRadialDamage (Variables|Default|GetDamage) (Transformation|GetActorLocation) (Variables|Default|GetDamageRadius) 0 0 self (Game|GetInstigatorController) true "ECC_WorldStatic")
  (Actor|DestroyActor))