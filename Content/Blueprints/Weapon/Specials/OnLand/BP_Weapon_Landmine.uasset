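; Landmine weapon special that explodes when a player character the game mode allows it to damage enters its overlap component.
; The overlap is handled only on the server, which asks the game mode with the victim's and instigator's controllers before detonating.
; Detonation applies full radial damage credited to the instigator, then destroys the actor.
; Clients spawn the explosion particles when the actor is destroyed, so no separate effect RPC is used.
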(event OnComponentBeginOverlap(r)
  (params (OverlappedComponent :type Primitive%20Component%20Object%20Reference) (OtherActor :type Actor%20Object%20Reference) (OtherComp :type Primitive%20Component%20Object%20Reference) (OtherBodyIndex :type Integer) (bFromSweep :type Boolean) (SweepResult :type Hit%20Result%20Structure%20%28by%20ref%29))
  (Networking|SwitchHasAuthority
    (:Authority
      (bind _asbp_player_character (Utilities|Casting|CastToBP_PlayerCharacter OtherActor))
      (if (Default|ShouldDamagePlayer? (.AsBP%20Player%20Game%20Mode (Utilities|Casting|CastToBP_PlayerGameMode (Game|GetGameMode))) (.AsBP%20Player%20Controller (Utilities|Casting|CastToBP_PlayerController (Pawn|GetController _asbp_player_character))) (.AsBP%20Player%20Controller (Utilities|Casting|CastToBP_PlayerController (Game|GetInstigatorController))))
        (CallFunction|Explosion)))))

(event EventBeginPlay)

(event Collision|EventActorBeginOverlap
  (params (OtherActor :type Actor%20Object%20Reference)))

(event EventTick
  (params (DeltaSeconds :type Float%20%28single-precision%29)))

(event EventDestroyed
  (|CallParentFunction)
  (Networking|SwitchHasAuthority
    (:Remote
      (Effects|SpawnEmitteratLocation "/Game/StarterContent/Particles/P_Explosion.P_Explosion" (Transformation|GetActorLocation)))))

(fn ConstructionScript)

(fn Explosion
  (Game|Damage|ApplyRadialDamage (Variables|Default|GetDamage) (+ (Transformation|GetActorLocation) "0, 0,2.000000") (Variables|Default|GetDamageRadius) 0 0 self (Game|GetInstigatorController) true "ECC_WorldStatic")
  (Actor|DestroyActor))