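; BP_Turret is a placed weapon that automatically damages enemy player characters entering its detection sphere.
; Targets exclude the instigator and, in team game modes, teammates; when the target leaves, it picks another overlapping one.
; A looping timer applies damage directly to the target, without projectiles or traces.
; Clients destroy the sphere, leaving detection to the server, and only they rotate the yaw and pitch components toward the target.
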(event OnComponentBeginOverlap(Sphere)
  (params (OverlappedComponent :type Primitive%20Component%20Object%20Reference) (OtherActor :type Actor%20Object%20Reference) (OtherComp :type Primitive%20Component%20Object%20Reference) (OtherBodyIndex :type Integer) (bFromSweep :type Boolean) (SweepResult :type Hit%20Result%20Structure%20%28by%20ref%29))
  (bind _asbp_player_character (Utilities|Casting|CastToBP_PlayerCharacter OtherActor))
  (Variables|Default|GetTarget
    (:then)
    (:else
      (if (CallFunction|ShouldDamageCharacter _asbp_player_character)
        (Variables|Default|SetTarget _asbp_player_character)
        (CallFunction|StartShoot)))))

(event OnComponentEndOverlap(Sphere)
  (params (OverlappedComponent :type Primitive%20Component%20Object%20Reference) (OtherActor :type Actor%20Object%20Reference) (OtherComp :type Primitive%20Component%20Object%20Reference) (OtherBodyIndex :type Integer))
  (if (== OtherActor (Variables|Default|GetTarget))
    (Variables|Default|SetTarget 0)
    (CallFunction|StopShooting)
    (CallFunction|SetNewTarget)))

(event EventBeginPlay
  (|CallParentFunction)
  (Networking|SwitchHasAuthority
    (:Remote
      (Components|DestroyComponent (Variables|Default|GetSphere)))))

(event EventTick
  (params (DeltaSeconds :type Float%20%28single-precision%29))
  (|CallParentFunction DeltaSeconds)
  (Networking|SwitchHasAuthority
    (:Remote
      (bind _target (Variables|Default|GetTarget)
        (:then
          (Transformation|SetWorldRotation (Variables|Default|GetYawTurning) (Math|Rotator|MakeRotator 0.0 0.0 (.yaw (Math|Rotator|FindLookatRotation (Transformation|GetWorldLocation (Variables|Default|GetPitchTurning)) (Transformation|GetActorLocation _target)))) false false)
          (Transformation|SetRelativeRotation (Variables|Default|GetPitchTurning) (Math|Rotator|MakeRotator 0.0 (.pitch (Math|Rotator|FindLookatRotation (Transformation|GetWorldLocation (Variables|Default|GetPitchTurning)) (Transformation|GetActorLocation _target))) 0.0) false false))
        (:else)))))

(fn ConstructionScript
  (|CallParentFunction))

(fn ShouldDamageCharacter
  (params (Character :type BP%20Player%20Character%20Object%20Reference))
  (bind _instigator (Variables|Default|GetInstigator)
    (:then
      (if (== _instigator Character)
        (return false)
        (else
          (Utilities|Casting|CastToBP_TeamGameMode (Game|GetGameMode)
            (:then
              (return (CallFunction|IsAnotherTeam? (Game|GetInstigatorController) (Pawn|GetController Character))))
            (:CastFailed
              (return true))))))
    (:else
      (return true))))

(fn IsAnotherTeam?
  (params (Player :type Controller%20Object%20Reference) (OtherPlayer :type Controller%20Object%20Reference))
  (return (!= (Variables|/Game/Blueprints/Game/BP_TeamPlayerState.BP_TeamPlayerState_C|GetTeam (.AsBP%20Team%20Player%20State (Utilities|Casting|CastToBP_TeamPlayerState (Variables|/Script/Engine.Controller|GetPlayerState Player)))) (Variables|/Game/Blueprints/Game/BP_TeamPlayerState.BP_TeamPlayerState_C|GetTeam (.AsBP%20Team%20Player%20State (Utilities|Casting|CastToBP_TeamPlayerState (Variables|/Script/Engine.Controller|GetPlayerState OtherPlayer)))))))

(fn SetNewTarget
  (for _array_element (Collision|GetOverlappingActors "/Game/Blueprints/Players/BP_PlayerCharacter.BP_PlayerCharacter_C" :!class /Script/Engine.Actor)
    (if (CallFunction|ShouldDamageCharacter (.AsBP%20Player%20Character (Utilities|Casting|CastToBP_PlayerCharacter _array_element)))
      (Variables|Default|SetTarget (.AsBP%20Player%20Character (Utilities|Casting|CastToBP_PlayerCharacter _array_element)))
      (CallFunction|StartShoot)
      (return))))

(fn Shoot
  (bind _target (Variables|Default|GetTarget)
    (:then
      (Game|Damage|ApplyDamage _target (Variables|Default|GetDamage) (Game|GetInstigatorController) self))
    (:else)))

(fn StartShoot
  (bind _returnvalue (Utilities|Time|SetTimerbyFunctionName 0 "Shoot" (Variables|Default|GetShootDelay) true))
  (Variables|Default|SetShootTimer _returnvalue))

(fn StopShooting
  (Utilities|Time|ClearandInvalidateTimerbyHandle (Variables|Default|GetShootTimer)))