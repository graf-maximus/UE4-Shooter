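; Networked firearm Blueprint that extends a parent weapon with shooting, spread, recoil and timed reloading.
; On authority, each use spawns the projectile class if set, otherwise line-traces from the player camera for point damage, with random spread around the owner's forward vector.
; The Reloading RepNotify starts the server's ammo refill timer, also triggered by firing on empty.
; Remote instances play timeline-driven pitch recoil for the local controller.
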(event Custom|DEBUG_DRAW
  (params (Start :type Vector) (End :type Vector) (Hit :type Vector))
  (Rendering|Debug|DrawDebugLine Start End "(R=1.000000,G=0.233938,B=0.000000,A=1.000000)" 5.0 2.0)
  (Rendering|Debug|DrawDebugSphere Hit 4e+01 12 "(R=1.000000,G=0.000000,B=0.005026,A=1.000000)" 5.0 2.0))

(event EventPlayWeaponEffects
  (|Playrecoilanim))

(fn ConstructionScript
  (|CallParentFunction))

(fn UseWeapon
  (bind _used (|CallParentFunction))
  (if _used
    (Networking|SwitchHasAuthority
      (:Authority
        (if (Utilities|IsValidClass (Variables|Default|GetFireProjectile))
          (CallFunction|SpawnShootProjectile)
          (return true)
          (else
            (CallFunction|ShootFireTrace)
            (return true))))
      (:Remote
        (CallFunction|PlayWeaponEffects)))
    (else
      (Networking|SwitchHasAuthority
        (:Authority
          (if (and (<= (Variables|Default|GetCurrentAmmo) 0) (> (Variables|Default|GetTotalAmmo) 0))
            (Variables|Default|SetReloading true)
            (return false)
            (else
              _)))
        (:Remote
          _))
      (return false))))

(fn ShootFireTrace
  (bind _asbp_player_character (Utilities|Casting|CastToBP_PlayerCharacter (Game|GetInstigator))
    (:then
      (bind _outhit (Collision|LineTraceForObjects (Transformation|GetWorldLocation (Variables|/Game/Blueprints/Players/BP_PlayerCharacter.BP_PlayerCharacter_C|GetCamera _asbp_player_character)) (+ (Transformation|GetWorldLocation (Variables|/Game/Blueprints/Players/BP_PlayerCharacter.BP_PlayerCharacter_C|GetCamera _asbp_player_character)) (* (CallFunction|GetRotateBullet) 10000)) (Utilities|Array|MakeArray "ObjectTypeQuery1" "ObjectTypeQuery2" "ObjectTypeQuery3") false (Utilities|Array|MakeArray self (Game|GetInstigator)) "None"))
      (Game|Damage|ApplyPointDamage (.HitActor (Collision|BreakHitResult _outhit)) (Variables|Default|GetDamage) (Math|Vector|GetUnitDirection(Vector) (.TraceEnd (Collision|BreakHitResult _outhit)) (.TraceStart (Collision|BreakHitResult _outhit))) _outhit (Game|GetInstigatorController) self))
    (:CastFailed
      (return))))

(fn ReloadFinished
  (Variables|Default|SetReloading false)
  (Variables|Default|SetCurrentAmmo (+ (Variables|Default|GetAmmoToReload) (Variables|Default|GetCurrentAmmo)))
  (Variables|Default|SetTotalAmmo (- (Variables|Default|GetTotalAmmo) (Variables|Default|GetAmmoToReload))))

(fn OnRepReloading
  (Networking|SwitchHasAuthority
    (:Authority
      (if (Variables|Default|GetReloading)
        (if (CallFunction|AbletoReload)
          (Utilities|Time|SetTimerbyFunctionName 0 "ReloadFinished" (Variables|Default|GetReloadTime))
          (Variables|Default|SetAmmoToReload (Math|Integer|Min(Integer) (- (.CurrentAmmo (Utilities|GetClassDefaults "BP_FireWeapons_C")) (Variables|Default|GetCurrentAmmo)) (Variables|Default|GetTotalAmmo)))
          (else
            (Variables|Default|SetReloading false)))))))

(fn AbletoReload
  (return (Math|Boolean|ANDBoolean (< (Variables|Default|GetCurrentAmmo) (.CurrentAmmo (Utilities|GetClassDefaults "BP_FireWeapons_C"))) (> (Variables|Default|GetTotalAmmo) 0) (not (Class|KismetSystemLibrary|IsTimerActive 0 "ReloadFinished")))))

(fn AbletoUseWeapon
  (return (and (|CallParentFunction) (not (Variables|Default|GetReloading)))))

(fn SpawnShootProjectile
  (bind _asbp_player_character (Utilities|Casting|CastToBP_PlayerCharacter (Game|GetInstigator)))
  (Game|SpawnActorfromClass (Variables|Default|GetFireProjectile) (Math|Transform|MakeTransform (+ (Transformation|GetWorldLocation (Variables|/Game/Blueprints/Players/BP_PlayerCharacter.BP_PlayerCharacter_C|GetCamera _asbp_player_character)) (* (Transformation|GetActorForwardVector (Components|GetOwner)) 50)) (Math|Conversions|RotationFromXVector (CallFunction|GetRotateBullet)) "1,1,1") "AlwaysSpawn" self (Variables|Default|GetDamage) (Game|GetInstigator)))

(fn GetRotateBullet
  (bind _returnvalue (Components|GetOwner))
  (bind _spreadangle (Variables|Default|GetSpreadAngle))
  (bind _spreadangle_2 (Variables|Default|GetSpreadAngle))
  (return (Math|Vector|RotateVectorAroundAxis (Math|Vector|RotateVectorAroundAxis (Transformation|GetActorForwardVector _returnvalue) (Math|Random|RandomFloatinRange (* -1 _spreadangle_2) _spreadangle_2) (Transformation|GetActorRightVector _returnvalue)) (Math|Random|RandomFloatinRange (* -1 _spreadangle) _spreadangle) (Transformation|GetActorUpVector _returnvalue))))

(fn ReloadWeapon
  (if (not (Variables|Default|GetReloading))
    (Variables|Default|SetReloading true)))