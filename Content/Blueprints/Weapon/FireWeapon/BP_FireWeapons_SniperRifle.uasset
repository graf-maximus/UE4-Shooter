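; Sniper rifle Blueprint, a child fire weapon that uses its secondary action as a zoomed aim.
; The client secondary-use event toggles the aiming state on press and switches the owner's camera between narrow and normal field of view for the local player only.
; The secondary action extends the parent logic to remove spread while aiming, and stopping it restores spread from the class defaults.
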(event EventUseSecondaryAction
  (|CallParentFunction)
  (if (Variables|Default|GetUsingSecondary)
    (Variables|Default|SetSpreadAngle 0.0)))

(event EventStopUseSecondaryAction
  (|CallParentFunction)
  (Variables|Default|SetSpreadAngle (Utilities|GetClassDefaults (Utilities|GetClass self))))

(event EventClient-UseSecondary
  (params (Use :type Boolean))
  (if Use
    (Variables|Default|SetUsingSecondary (not (Variables|Default|GetUsingSecondary)))
    (if (Pawn|IsLocalPlayerController (Game|GetInstigatorController))
      (Camera|SetFieldOfView (Variables|/Game/Blueprints/Players/BP_PlayerCharacter.BP_PlayerCharacter_C|GetCamera (Variables|Default|GetWeaponOwner)) (Math|Float|SelectFloat 15.0 9e+01 (Variables|Default|GetUsingSecondary))))))

(fn ConstructionScript
  (|CallParentFunction))