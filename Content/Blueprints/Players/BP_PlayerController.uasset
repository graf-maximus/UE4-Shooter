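; Player controller that handles HUD input, chat, map voting and timed respawns for each player.
; Tab swaps the main HUD for the tab menu while held, and T opens chat on the HUD.
; Server events forward chat messages and map votes to GameState components with the PlayerState.
; LaunchRespawnTimer schedules Respawn through the game mode and binds to match end, which clears the timer.
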(event Custom|SendMessageOnServer
  (params (Message :type Text))
  ;[1 1 1] Send message on server
  (Default|PrintMessage (Variables|/Game/Blueprints/Game/BP_GameStateBase.BP_GameStateBase_C|GetBP_ChatComponents (.AsBP%20Game%20State%20Base (Utilities|Casting|CastToBP_GameStateBase (Game|GetGameState)))) Message (.AsBP%20Player%20State (Utilities|Casting|CastToBP_PlayerState (Variables|GetPlayerState)))))

(event Custom|RoundEndedInRespawn
  (params (StopReason :type String))
  ;[1 1 1] Clear timer when round ended
  (EventDispatchers|UnbindEventfromMatchEnded (.AsBP%20Player%20Game%20Mode (Utilities|Casting|CastToBP_PlayerGameMode (Game|GetGameMode))) (delegate Custom|RoundEndedInRespawn))
  (Utilities|Time|ClearandInvalidateTimerbyHandle (Variables|Default|GetRespawnTimer)))

(event Custom|SendVoteOnServer
  (params (MapIndex :type Integer))
  ;[1 1 1] Send map vote to server
  (Default|SetVote (Variables|/Game/Blueprints/Game/BP_GameStateBase.BP_GameStateBase_C|GetBP_MapVoteComponent (.AsBP%20Game%20State%20Base (Utilities|Casting|CastToBP_GameStateBase (Game|GetGameState)))) MapIndex (.AsBP%20Player%20State (Utilities|Casting|CastToBP_PlayerState (Variables|GetPlayerState)))))

(event EventBeginPlay
  (Input|SetInputModeGameOnly self))

(event Input|KeyboardEvents|Tab
  (params (Key :type Key%20Structure :default "None"))
  (bind _returnvalue (HUD|GetHUD))
  (bind _asbp_main_hud (Utilities|Casting|CastToBP_MainHUD _returnvalue))
  ;[1 1 1] Show tab menu
  (:Pressed
    (Default|ToggleTabMenu _asbp_main_hud true)
    (Default|ToggleMainHUD _asbp_main_hud false))
  (:Released
    (Default|ToggleTabMenu _asbp_main_hud false)
    (Default|ToggleMainHUD _asbp_main_hud true)))

(event Input|KeyboardEvents|T
  (params (Key :type Key%20Structure :default "None"))
  ;[1 1 1] Activate chat
  (:Pressed
    (Default|ToggleSpeakChat (.AsBP%20Main%20HUD (Utilities|Casting|CastToBP_MainHUD (HUD|GetHUD))) true)))

(fn ConstructionScript)

(fn Respawn
  (bind _asbp_player_game_mode (Utilities|Casting|CastToBP_PlayerGameMode (Game|GetGameMode)))
  (Default|SpawnPlayer _asbp_player_game_mode self))

(fn LaunchRespawnTimer
  (params (Time :type Float%20%28single-precision%29))
  (bind _returnvalue (Utilities|Time|SetTimerbyFunctionName 0 "Respawn" Time))
  (Variables|Default|SetRespawnTimer _returnvalue)
  (EventDispatchers|BindEventtoMatchEnded (.AsBP%20Player%20Game%20Mode (Utilities|Casting|CastToBP_PlayerGameMode (Game|GetGameMode))) (EventDispatchers|CreateEvent :!event Custom|RoundEndedInRespawn)))